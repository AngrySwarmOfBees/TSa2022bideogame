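; Procedural maze actor that builds a seeded grid maze for a ball game on BeginPlay or Rebuild.
; GenerateMaze carves paths by randomized depth-first search with backtracking, using two-tile steps joined by bridge tiles and recording dead ends.
; SpawnMazeMeshes sends wall and wall-top instances to InstanceManager, which also supplies the actor's transform.
; The MazeBall spawns at a random dead end, and a fixed-seed dead-end pick becomes the InstanceManager endpoint.
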(event Custom|Rebuild
  (bind _returnvalue (Math|Random|MakeRandomStream 0))
  (bind _tilesize (Variables|Default|GetTileSize))
  (bind _tilesize_2 (Variables|Default|GetTileSize))
  (Transformation|SetActorTransform (Transformation|GetActorTransform (Variables|Default|GetInstanceManager)))
  (Class|BPIInstanceManager|RemoveAllInstances(Message) (Variables|Default|GetInstanceManager))
  (bind (_path_tiles _end_paths) (CallFunction|GenerateMaze (Variables|Default|GetSize) (Variables|Default|GetSeed)))
  (Variables|Default|SetPath%20Tiles%20Out _path_tiles)
  (bind _output_get (Variables|Default|SetEnd%20Paths%20Out _end_paths))
  (CallFunction|SpawnMazeMeshes)
  (bind _result (Utilities|Set|ToArray _output_get))
  (bind _returnvalue_2 (AddComponent|AddChildActorComponent false (Math|Transform|MakeTransform (Math|Vector|MakeVector (* (.X (Utilities|Struct|BreakIntPoint (.OutItem (Utilities|Array|Random _result)))) _tilesize) (* (.Y (Utilities|Struct|BreakIntPoint (.OutItem (Utilities|Array|Random _result)))) _tilesize) 4e+02) "0, 0, 0" "0.750000,0.750000,0.750000")))
  (Variables|Default|SetTransform (Transformation|GetWorldTransform _returnvalue_2))
  (Components|DestroyComponent _returnvalue_2)
  (bind _returnvalue_3 (Game|SpawnActorfromClass "/Game/orb/Procedural/MazeBall.MazeBall_C" (Variables|Default|GetTransform) "Undefined" self 0 0))
  (Variables|/Game/orb/Procedural/BP_instanceManager.BP_instanceManager_C|SetBall (Variables|Default|GetInstanceManager) _returnvalue_3)
  (Variables|/Game/orb/Procedural/MazeBall.MazeBall_C|SetInstanceManager _returnvalue_3 (Variables|Default|GetInstanceManager))
  (bind _result_2 (Utilities|Set|ToArray (Variables|Default|GetEnd%20Paths%20Out)))
  (Class|KismetMathLibrary|SeedRandomStream _returnvalue)
  (bind _returnvalue_4 (AddComponent|AddStaticMeshComponent false (Math|Transform|MakeTransform (Math|Vector|MakeVector (* (.X (Utilities|Struct|BreakIntPoint (.OutItem (Utilities|Array|RandomFromStream _result_2 _returnvalue)))) _tilesize_2) (* (.Y (Utilities|Struct|BreakIntPoint (.OutItem (Utilities|Array|RandomFromStream _result_2 _returnvalue)))) _tilesize_2) 2e+02))))
  (Variables|Default|SetEndLoc (Transformation|GetWorldTransform _returnvalue_4))
  (Components|DestroyComponent _returnvalue_4)
  (Default|AddEndpoint (Variables|Default|GetInstanceManager) (Variables|Default|GetEndLoc)))

(event EventBeginPlay
  (bind _returnvalue (Math|Random|MakeRandomStream 0))
  (bind _tilesize (Variables|Default|GetTileSize))
  (bind _tilesize_2 (Variables|Default|GetTileSize))
  (Transformation|SetActorTransform (Transformation|GetActorTransform (Variables|Default|GetInstanceManager)))
  (Class|BPIInstanceManager|RemoveAllInstances(Message) (Variables|Default|GetInstanceManager))
  (bind (_path_tiles _end_paths) (CallFunction|GenerateMaze (Variables|Default|GetSize) (Variables|Default|GetSeed)))
  (Variables|Default|SetPath%20Tiles%20Out _path_tiles)
  (bind _output_get (Variables|Default|SetEnd%20Paths%20Out _end_paths))
  (CallFunction|SpawnMazeMeshes)
  (bind _result (Utilities|Set|ToArray _output_get))
  (bind _returnvalue_2 (AddComponent|AddChildActorComponent false (Math|Transform|MakeTransform (Math|Vector|MakeVector (* (.X (Utilities|Struct|BreakIntPoint (.OutItem (Utilities|Array|Random _result)))) _tilesize) (* (.Y (Utilities|Struct|BreakIntPoint (.OutItem (Utilities|Array|Random _result)))) _tilesize) 4e+02) "0, 0, 0" "0.750000,0.750000,0.750000")))
  (Variables|Default|SetTransform (Transformation|GetWorldTransform _returnvalue_2))
  (Components|DestroyComponent _returnvalue_2)
  (bind _returnvalue_3 (Game|SpawnActorfromClass "/Game/orb/Procedural/MazeBall.MazeBall_C" (Variables|Default|GetTransform) "Undefined" self 0 0))
  (Variables|/Game/orb/Procedural/BP_instanceManager.BP_instanceManager_C|SetBall (Variables|Default|GetInstanceManager) _returnvalue_3)
  (Variables|/Game/orb/Procedural/MazeBall.MazeBall_C|SetInstanceManager _returnvalue_3 (Variables|Default|GetInstanceManager))
  (bind _result_2 (Utilities|Set|ToArray (Variables|Default|GetEnd%20Paths%20Out)))
  (Class|KismetMathLibrary|SeedRandomStream _returnvalue)
  (bind _returnvalue_4 (AddComponent|AddStaticMeshComponent false (Math|Transform|MakeTransform (Math|Vector|MakeVector (* (.X (Utilities|Struct|BreakIntPoint (.OutItem (Utilities|Array|RandomFromStream _result_2 _returnvalue)))) _tilesize_2) (* (.Y (Utilities|Struct|BreakIntPoint (.OutItem (Utilities|Array|RandomFromStream _result_2 _returnvalue)))) _tilesize_2) 2e+02))))
  (Variables|Default|SetEndLoc (Transformation|GetWorldTransform _returnvalue_4))
  (Components|DestroyComponent _returnvalue_4)
  (Default|AddEndpoint (Variables|Default|GetInstanceManager) (Variables|Default|GetEndLoc)))

(event EventTick
  (params (DeltaSeconds :type Float%20%28single-precision%29)))

(event EventEndPlay
  (params (EndPlayReason :type EEndPlayReason%20Enum :default "Destroyed"))
  (Class|BPIInstanceManager|RemoveAllInstances(Message) (Variables|Default|GetInstanceManager)))

(fn ConstructionScript
  (Transformation|SetActorTransform (Transformation|GetActorTransform (Variables|Default|GetInstanceManager)))
  (Class|BPIInstanceManager|RemoveAllInstances(Message) (Variables|Default|GetInstanceManager))
  (Variables|Default|SetSize (Utilities|Struct|MakeIntPoint (* (/ (.x (Variables|Default|GetSize)) 2) 2) (* (/ (.y (Variables|Default|GetSize)) 2) 2)))
  (bind (_path_tiles _end_paths) (CallFunction|GenerateMaze (Variables|Default|GetSize) (Variables|Default|GetSeed)))
  (Variables|Default|SetPath%20Tiles%20Out _path_tiles)
  (Variables|Default|SetEnd%20Paths%20Out _end_paths))

(fn GenerateMaze
  (params (size :type Int%20Point%20Structure%20%28by%20ref%29) (Seed :type Integer))
  (bind _randstream (LocalVariables|GetRandStream))
  (Math|Random|SetRandomStreamSeed _randstream Seed)
  (bind _output_get (LocalVariables|SetL_size size))
  (bind _output_get_2 (LocalVariables|SetStartingLoc (Utilities|GetRandLocation _output_get _randstream)))
  (bind _output_get_3 (Variables|Default|SetStartingLocation _output_get_2))
  (bind _output_get_4 (LocalVariables|SetCurrentLoc _output_get_3))
  (Class|KismetMathLibrary|SeedRandomStream (LocalVariables|GetRandStream))
  (CallFunction|AddNeigbhborLoc size (LocalVariables|GetRandStream) _output_get_4 (Variables|Default|GetPath%20Tiles) (Variables|Default|GetBridge%20Tiles) (Variables|Default|GetTo%20Check) (Variables|Default|GetEnd%20Paths) :!label _label)
  (if (> (Utilities|Set|Length (Variables|Default|GetTo%20Check)) 0)
    (CallFunction|BackTrack (LocalVariables|GetCurrentLoc) (Variables|Default|GetTo%20Check) (Variables|Default|GetBridge%20Tiles) (Variables|Default|GetPath%20Tiles))
    (goto _label)
    (else
      (return (Variables|Default|GetPath%20Tiles) (Variables|Default|GetEnd%20Paths)))))

(fn AddNeigbhborLoc
  (params (Size :type Int%20Point%20Structure%20%28by%20ref%29) (RandStream :type Random%20Stream%20Structure%20%28by%20ref%29) (CurrentLoc :type Int%20Point%20Structure%20%28by%20ref%29) (PathTiles :type Set%20of%20Int%20Point%20Structures) (BridgeTiles :type Set%20of%20Int%20Point%20Structures) (ToCheck :type Set%20of%20Int%20Point%20Structures) (EndPaths :type Set%20of%20Int%20Point%20Structures))
  (Class|KismetMathLibrary|SeedRandomStream RandStream)
  (LocalVariables|SetNeighborIndex (Math|Random|RandomIntegerinRangefromStream 0 3 RandStream))
  (if (Utilities|CheckIsValidLocation (.Floor (Utilities|GetNeighborandBridge CurrentLoc (LocalVariables|GetNeighborIndex))) Size PathTiles BridgeTiles) :!label _label
    (Utilities|Set|Add PathTiles (.Floor (Utilities|GetNeighborandBridge CurrentLoc (LocalVariables|GetNeighborIndex))))
    (Utilities|Set|Add BridgeTiles (.Bridge (Utilities|GetNeighborandBridge CurrentLoc (LocalVariables|GetNeighborIndex))))
    (Utilities|Set|Add ToCheck (.Floor (Utilities|GetNeighborandBridge CurrentLoc (LocalVariables|GetNeighborIndex))))
    (CallFunction|AddNeigbhborLoc Size RandStream (.Floor (Utilities|GetNeighborandBridge CurrentLoc (LocalVariables|GetNeighborIndex))) PathTiles BridgeTiles ToCheck EndPaths)
    (else
      (Utilities|DoN+ 4
        (:Exit
          (LocalVariables|SetNeighborIndex (Math|Integer|SelectInt 0 (+ (LocalVariables|GetNeighborIndex) 1) (>= (+ (LocalVariables|GetNeighborIndex) 1) 4)))
          (goto _label))
        (:Over%20Nth
          (bind _count (CallFunction|GetNeighborCount CurrentLoc PathTiles))
          (if (== _count 1)
            (Utilities|Set|Add (Variables|Default|GetEnd%20Paths) CurrentLoc)))))))

(fn GetNeighborCount
  (params (CurrentLoc :type Int%20Point%20Structure%20%28by%20ref%29) (PathTiles :type Set%20of%20Int%20Point%20Structures))
  (for _array_element (Utilities|GetNeighborLocation CurrentLoc 1)
    (if (Utilities|Set|Contains PathTiles _array_element)
      (Math|Integer|IncrementInt (LocalVariables|GetCounter))))
  (return (LocalVariables|GetCounter)))

(fn BackTrack
  (params (Current%20Tile :type Int%20Point%20Structure%20%28by%20ref%29) (To%20check :type Set%20of%20Int%20Point%20Structures) (Bridge%20Tiles :type Set%20of%20Int%20Point%20Structures) (Path%20Tiles :type Set%20of%20Int%20Point%20Structures))
  (bind _result (Utilities|Set|ToArray To%20check))
  (|SetBy-RefVar Current%20Tile (Utilities|Array|Get(acopy) _result (Utilities|Array|LastIndex _result)))
  (bind _returnvalue (Utilities|Set|Remove To%20check (Utilities|Array|Get(acopy) _result (Utilities|Array|LastIndex _result))))
  (if _returnvalue
    (bind _result_2 (Utilities|Set|ToArray Bridge%20Tiles))
    (if (not (<= (Utilities|Array|LastIndex _result_2) 0))
      (Utilities|Set|Add Path%20Tiles (Utilities|Array|Get(acopy) _result_2 (Utilities|Array|LastIndex _result_2)))
      (bind _returnvalue_2 (Utilities|Set|Remove Bridge%20Tiles (Utilities|Array|Get(acopy) _result_2 (Utilities|Array|LastIndex _result_2))))
      (if (not _returnvalue_2)
        (Development|PrintString "bridge tile removal failed")))
    (else
      (Development|PrintString "To check removal failed"))))

(fn SpawnMazeMeshes
  (bind _size (Variables|Default|GetSize))
  (bind _size_2 (Variables|Default|GetSize))
  (for _index (range 0 (.x _size))
    (for _index_2 (range 0 (.y _size))
      (bind _output_get (LocalVariables|SetLoop%20Loc (Utilities|Struct|MakeIntPoint _index _index_2)))
      (if (Utilities|Set|Contains (Variables|Default|GetPath%20Tiles%20Out) _output_get)
        (for (_array_element _array_index) (Utilities|GetNeighborLocation (LocalVariables|GetLoop%20Loc) 1)
          (bind _output_get_2 (LocalVariables|SetLoop%20Index _array_index))
          (Utilities|Array|SetArrayElem (LocalVariables|GetSegmentIndex) _output_get_2 (Utilities|Set|Contains (Variables|Default|GetPath%20Tiles%20Out) _array_element) true)
          (if (not (Utilities|Set|Contains (Variables|Default|GetPath%20Tiles%20Out) _array_element))
            (Class|BPIInstanceManager|AddNewMeshInstance(Message) (Variables|Default|GetInstanceManager) (Variables|Default|GetWall%20mesh) (Math|Transform|MakeTransform (.Location (Math|Transform|BreakTransform (Utilities|BuildTileLoc (LocalVariables|GetLoop%20Loc) 0.0 (LocalVariables|GetLoop%20Index)))) (Math|Rotator|MakeRotator (.Roll (Math|Rotator|BreakRotator (.Rotation (Math|Transform|BreakTransform (Utilities|BuildTileLoc (LocalVariables|GetLoop%20Loc) 0.0 (LocalVariables|GetLoop%20Index)))))) (.Pitch (Math|Rotator|BreakRotator (.Rotation (Math|Transform|BreakTransform (Utilities|BuildTileLoc (LocalVariables|GetLoop%20Loc) 0.0 (LocalVariables|GetLoop%20Index)))))) (.Yaw (Math|Rotator|BreakRotator (.Rotation (Math|Transform|BreakTransform (Utilities|BuildTileLoc (LocalVariables|GetLoop%20Loc) 0.0 (LocalVariables|GetLoop%20Index))))))) (Variables|Default|Getwallscale)))))
        (else
          (Class|BPIInstanceManager|AddNewMeshInstance(Message) (Variables|Default|GetInstanceManager) (Variables|Default|GetWall%20Top) (Utilities|BuildTileLoc (LocalVariables|GetLoop%20Loc) 1e+02)))))
    (for _index_3 (range 0 (.x _size_2))
      (Class|BPIInstanceManager|AddNewMeshInstance(Message) (Variables|Default|GetInstanceManager) (Variables|Default|GetWall%20Top) (Utilities|BuildTileLoc (Utilities|Struct|MakeIntPoint (+ _index_3 1) 0) 1e+02)))
    (for _index_4 (range 0 (.x _size_2))
      (Class|BPIInstanceManager|AddNewMeshInstance(Message) (Variables|Default|GetInstanceManager) (Variables|Default|GetWall%20Top) (Utilities|BuildTileLoc (Utilities|Struct|MakeIntPoint (+ _index_4 -1) (* (.y _size_2) 1)) 1e+02)))))

(fn AddNewMeshInstance
  (params (MeshType :type Static%20Mesh%20Object%20Reference) (Transform :type Transform))
  (return false 0))

(fn RemoveAllInstances
  (return false))

(fn RemoveAllMeshInstances
  (params (Mesh :type Static%20Mesh%20Object%20Reference))
  (return false))

(fn RemoveMeshInstance
  (params (Mesh :type Static%20Mesh%20Object%20Reference) (Index :type Integer))
  (return false))

(fn RotateMaze
  (for _array_element (LocalVariables|GetBoxes)
    (Components|DestroyComponent _array_element))
  (for _index (range 0 (Components|InstancedStaticMesh|GetInstanceCount (Variables|Default|GetInstancedStaticMesh)))
    (bind _returnvalue (AddComponent|AddBoxComponent false (.OutInstanceTransform (Components|InstancedStaticMesh|GetInstanceTransform (Variables|Default|GetInstancedStaticMesh) _index true))))
    (Utilities|Array|Add (LocalVariables|GetBoxes) _returnvalue))
  (return false))